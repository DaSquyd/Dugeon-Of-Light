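; PadController_BP is the completion checker for the Lights Out puzzle, watching a set of pads.
; Every tick it scans the Pads array and treats the puzzle as solved only when every pad's IsOn is true.
; While solved, it sets LightsOutComplete on CustomGameMode and sends ToggleStateMessage(true) to each actor in AffectedActors, repeating each tick because nothing latches the result.
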(event `self.ReceiveTick`
  (params (DeltaSeconds :type "Float (single-precision)"))
  (set `self.AllOn` true)
  (for _array_element (`self.Pads`)
    (if (not (`/Game/Blueprints/LightsOut/LightsOut_Pad.isOn` _array_element))
      (set `self.AllOn` false)
      (break)))
  (if (`self.AllOn`)
    (bind _ascustom_game_mode (cast `/Game/Maps/CustomGameMode` (`GameplayStatics.GetGameMode`)))
    (set `/Game/Maps/CustomGameMode.LightsOutComplete` true _ascustom_game_mode)
    (for _array_element_2 (`self.affectedActors`)
      (message `/Game/Blueprints/ToggleInterface.ToggleState` _array_element_2 true))))

(fn `UserConstructionScript`)