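; Floor pad Blueprint for a Lights Out style puzzle, where stepping on a pad flips it and its neighbors.
; When a BP_Player begins overlapping its Box, it inverts its own IsOn flag and that of every pad in the AdjPads array.
; Tick reapplies the on or off material to the Cube every frame, so the visual follows changes made by other pads.
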(event `self.ReceiveTick`
  (params (DeltaSeconds :type "Float (single-precision)"))
  (bind _cube (`self.Cube`))
  (if (`self.isOn`)
    (`PrimitiveComponent.SetMaterial` _cube 0 "/Game/Blueprints/LightsOut/isOn.isOn")
    (else
      (`PrimitiveComponent.SetMaterial` _cube 0 "/Game/Blueprints/LightsOut/isOff.isOff"))))

(event `self.Box.OnComponentBeginOverlap`
  (params (OverlappedComponent :type "PrimitiveComponent Object Reference") (OtherActor :type "Actor Object Reference") (OtherComp :type "PrimitiveComponent Object Reference") (OtherBodyIndex :type Integer) (bFromSweep :type Boolean) (SweepResult :type "HitResult Structure (by ref)"))
  (if (== (`GameplayStatics.GetObjectClass` OtherActor) "/Game/Blueprints/Player/BP_Player(1).BP_Player_C")
    (if (`self.isOn`)
      (set `self.isOn` false)
      (else
        (set `self.isOn` true)))
    (for _array_element (`self.adjPads`)
      (if (`/Game/Blueprints/LightsOut/Pad.isOn` _array_element)
        (set `/Game/Blueprints/LightsOut/Pad.isOn` false _array_element)
        (else
          (set `/Game/Blueprints/LightsOut/Pad.isOn` true _array_element))))))

(fn `UserConstructionScript`)