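; KeyDoor is a door actor that opens by spending one of the player's DoorKeys.
; Tick casts and caches player pawn 0 as BP_Player each frame for the key check.
; Any actor overlap while that player has keys decrements DoorKeys, hides the Cube and disables its collision, without checking which actor overlapped.
; The construction script records InitialLocation, which the graphs shown never read.
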(event `self.ReceiveActorBeginOverlap`
  (params (OtherActor :type "Actor Object Reference"))
  (if (> (`/Game/Blueprints/Player/BP_Player.DoorKeys` (stale `self.ReceiveTick` _asbp_player)) 0)
    (bind _asbp_player (cast `/Game/Blueprints/Player/BP_Player` (`GameplayStatics.GetPlayerPawn` 0)))
    (set `/Game/Blueprints/Player/BP_Player.DoorKeys` (- (`/Game/Blueprints/Player/BP_Player.DoorKeys` _asbp_player) 1) _asbp_player)
    (`SceneComponent.SetVisibility` (`self.Cube`) false false)
    (`PrimitiveComponent.SetCollisionEnabled` (`self.Cube`) "NoCollision")))

(event `self.ReceiveTick`
  (params (DeltaSeconds :type "Float (single-precision)"))
  (bind _asbp_player (cast `/Game/Blueprints/Player/BP_Player` (`GameplayStatics.GetPlayerPawn` 0))))

(fn `UserConstructionScript`
  (bind _returnvalue (`self.K2_GetActorLocation`))
  (`self.K2_SetActorLocation` _returnvalue)
  (set `self.initialLocation` _returnvalue))