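; BossDoor is a door actor among the light objects that opens only when the boss key is held.
; When ToggleState turns on and HasBossKey is true, it hides its Cube and disables collision, with no branch to close it again.
; The construction script stores InitialLocation, used only by a disconnected timeline movement.
; A delayed load of the MicroPuzzle_BlockStack level is also left unconnected.
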(event `/Game/Blueprints/ToggleInterface.ToggleState`
  (params (OnOff :type Boolean))
  (if OnOff
    (if (`self.hasBossKey`)
      (`SceneComponent.SetVisibility` (`self.Cube`) false false)
      (`PrimitiveComponent.SetCollisionEnabled` (`self.Cube`) "NoCollision"))))

(fn `UserConstructionScript`
  (bind _returnvalue (`self.K2_GetActorLocation`))
  (`self.K2_SetActorLocation` _returnvalue)
  (set `self.initialLocation` _returnvalue))