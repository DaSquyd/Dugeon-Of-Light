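; AttackLight is a light object that cycles between red, green and blue when it takes damage.
; On BeginPlay it applies the material matching its current color to its static mesh.
; Any damage prints the amount, then advances the color and swaps the material.
; A SwitchLight event enters the same cycle logic without the print, so the color can also change without damage.
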(event `self.ReceiveBeginPlay`
  (`self.SetColor`))

(event `SetColor`
  (bind _staticmeshcomponent (`self.StaticMeshComponent`))
  ;[1 1 1] Set Colors
  (switch `/Game/Blueprints/LightObjects/ESwitchColors` (`self.CurrentColor`)
    (:`NewEnumerator0`
      (`PrimitiveComponent.SetMaterial` _staticmeshcomponent 0 "/Game/Materials/RedLight.RedLight"))
    (:`NewEnumerator1`
      (`PrimitiveComponent.SetMaterial` _staticmeshcomponent 0 "/Game/Materials/GreenLight.GreenLight"))
    (:`NewEnumerator2`
      (`PrimitiveComponent.SetMaterial` _staticmeshcomponent 0 "/Game/Materials/BlueLight.BlueLight"))))

(event `self.ReceiveAnyDamage`
  (params (Damage :type "Float (single-precision)") (DamageType :type "DamageType Object Reference") (InstigatedBy :type "Controller Object Reference") (DamageCauser :type "Actor Object Reference"))
  (bind _staticmeshcomponent (`self.StaticMeshComponent`))
  ;[1 1 1] Color Cycle
  (`KismetSystemLibrary.PrintString` (`KismetStringLibrary.Conv_DoubleToString` Damage))
  (switch `/Game/Blueprints/LightObjects/ESwitchColors` (`self.CurrentColor`) :!label _label
    (:`NewEnumerator0`
      (set `self.CurrentColor` "NewEnumerator1")
      (`PrimitiveComponent.SetMaterial` _staticmeshcomponent 0 "/Game/Materials/GreenLight.GreenLight"))
    (:`NewEnumerator1`
      (set `self.CurrentColor` "NewEnumerator2")
      (`PrimitiveComponent.SetMaterial` _staticmeshcomponent 0 "/Game/Materials/BlueLight.BlueLight"))
    (:`NewEnumerator2`
      (set `self.CurrentColor` "NewEnumerator0")
      (`PrimitiveComponent.SetMaterial` _staticmeshcomponent 0 "/Game/Materials/RedLight.RedLight"))))

(event `SwitchLight`
  ;[1 1 1] Color Cycle
  (goto _label))

(fn `UserConstructionScript`)