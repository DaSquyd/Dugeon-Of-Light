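; Door actor among the light objects that opens when it receives a ToggleState event with OnOff true.
; Opening is instant: it hides the Cube and SMCeilingB2 components and disables their collision, with no branch to close it again.
; The construction script caches the actor's starting location, which only a disconnected timeline movement uses.
; An unconnected delayed load of the MicroPuzzle_BlockStack level also remains in the graph.
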(event `/Game/Blueprints/ToggleInterface.ToggleState`
  (params (OnOff :type Boolean))
  (if OnOff
    (`SceneComponent.SetVisibility` (`self.Cube`) false false)
    (`PrimitiveComponent.SetCollisionEnabled` (`self.Cube`) "NoCollision")
    (`SceneComponent.SetVisibility` (`self.SM_Ceiling_B_2`) false false)
    (`PrimitiveComponent.SetCollisionEnabled` (`self.SM_Ceiling_B_2`) "NoCollision")))

(fn `UserConstructionScript`
  (bind _returnvalue (`self.K2_GetActorLocation`))
  (`self.K2_SetActorLocation` _returnvalue)
  (set `self.initialLocation` _returnvalue))