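; SubmitButton is an overlap-triggered button that checks a three-cube placement puzzle.
; When an actor other than BoxTrigger overlaps it, nested tests compare each cube's location to its stored target within a fixed tolerance.
; If all three match, it sends ToggleStateMessage(true) to every entry in AffectedActors.
; Only a failure on the third cube prints "fail"; earlier mismatches do nothing.
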(event `self.ReceiveActorBeginOverlap`
  (params (OtherActor :type "Actor Object Reference"))
  (if (!= "/Script/Engine.Actor" "/Game/Blueprints/LightObjects/BoxTrigger.BoxTrigger_C")
    (if (== (`self.locationCube1`) (`self.K2_GetActorLocation` (`self.Cube1`)) :`ErrorTolerance` 90.0)
      (if (== (`self.locationCube2`) (`self.K2_GetActorLocation` (`self.Cube2`)) :`ErrorTolerance` 90.0)
        (if (== (`self.locationCube3`) (`self.K2_GetActorLocation` (`self.Cube3`)) :`ErrorTolerance` 90.0)
          (for _array_element (`self.affectedActors`)
            (message `/Game/Blueprints/ToggleInterface.ToggleState` _array_element true))
          (else
            (`KismetSystemLibrary.PrintString` "fail")))))))

(fn `UserConstructionScript`)