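; StackBox3 is a physics box actor that drifts toward the player and snaps back to its starting spot when shot or damaged.
; It records its location at BeginPlay as the reset origin.
; Each tick within a short range of the first player controller, it applies a force to its Cube along the unnormalized vector toward that controller.
; Overlap with BP_Bullet or any damage teleports it to the origin with zeroed rotation.
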(event `self.ReceiveActorBeginOverlap`
  (params (OtherActor :type "Actor Object Reference"))
  (if (== (`GameplayStatics.GetObjectClass` OtherActor) "/Game/Blueprints/Projectile/BP_Bullet.BP_Bullet_C")
    (`self.K2_TeleportTo` (`self.Origin`))))

(event `self.ReceiveBeginPlay`
  (set `self.Origin` (`self.K2_GetActorLocation`)))

(event `self.ReceiveTick`
  (params (DeltaSeconds :type "Float (single-precision)"))
  (if (<= (`KismetMathLibrary.Vector_Distance` (`self.K2_GetActorLocation`) (`self.K2_GetActorLocation` (`GameplayStatics.GetPlayerController` 0))) 200.0)
    (`PrimitiveComponent.AddForce` (`self.Cube`) (- (`self.K2_GetActorLocation` (`GameplayStatics.GetPlayerController` 0)) (`self.K2_GetActorLocation`)) "None" false)))

(event `self.ReceiveAnyDamage`
  (params (Damage :type "Float (single-precision)") (DamageType :type "DamageType Object Reference") (InstigatedBy :type "Controller Object Reference") (DamageCauser :type "Actor Object Reference"))
  (`self.K2_TeleportTo` (`self.Origin`)))

(fn `UserConstructionScript`)