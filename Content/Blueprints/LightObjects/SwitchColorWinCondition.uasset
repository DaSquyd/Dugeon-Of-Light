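; Win-condition actor for a color-switch puzzle that opens two doors when every light matches the target color.
; Each Tick shows the target on an Indicator and polls the Lights array for a full match.
; A match randomizes all lights and advances the target through Blue, Red and Green.
; Matching Green sets Win, destroys both doors, and subsequent ticks destroy any remaining lights.
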(event `self.ReceiveTick`
  (params (DeltaSeconds :type "Float (single-precision)"))
  (if (`self.Win`)
    (for _array_element (`self.Lights`)
      (`/Engine/EditorBlueprintResources/StandardMacros.IsValid` _array_element
        (:`Is Valid`
          (`self.K2_DestroyActor` _array_element))))
    (else
      (set `/Game/Blueprints/LightObjects/AttackLight.CurrentColor` (`self.Color`) (`self.Indicator`))
      (`/Game/Blueprints/LightObjects/AttackLight.SetColor` (`self.Indicator`))
      (set `self.Success` true)
      (for _array_element_2 (`self.Lights`)
        (if (not (`|EnumEquality` (`/Game/Blueprints/LightObjects/AttackLight.CurrentColor` _array_element_2) (`self.Color`)))
          (set `self.Success` false)))
      (if (`self.Success`)
        (for _array_element_3 (`self.Lights`)
          (set `/Game/Blueprints/LightObjects/AttackLight.CurrentColor` (select `int` (`KismetMathLibrary.RandomIntegerInRange` 0 2) :`0` "NewEnumerator0" :`1` "NewEnumerator1" :`2` "NewEnumerator2" :!type "/Game/Blueprints/LightObjects/ESwitchColors Enum") _array_element_3)
          (`/Game/Blueprints/LightObjects/AttackLight.SetColor` _array_element_3))
        (switch `/Game/Blueprints/LightObjects/ESwitchColors` (`self.Color`)
          (:`NewEnumerator0`
            (set `self.Color` "NewEnumerator1"))
          (:`NewEnumerator1`
            (set `self.Win` true)
            (`KismetSystemLibrary.PrintString` "Puzzle Solved")
            (`self.K2_DestroyActor` (`self.Door 1`))
            (`self.K2_DestroyActor` (`self.Door 2`)))
          (:`NewEnumerator2`
            (set `self.Color` "NewEnumerator0")))))))

(fn `UserConstructionScript`)