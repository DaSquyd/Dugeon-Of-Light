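; Boss key pickup that floats and spins in the level until the player collects it.
; On overlap with BP_Player, it sets the boss key flag and key number on CustomGameMode, destroys itself and prints an on-screen message.
; Tick bobs the Cube mesh vertically with a looping cosine over a timed cycle while yawing it at a steady rotation speed.
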(event `self.ReceiveActorBeginOverlap`
  (params (OtherActor :type "Actor Object Reference"))
  (cast `/Game/Blueprints/Player/BP_Player` OtherActor)
  (bind _ascustom_game_mode (cast `/Game/Maps/CustomGameMode` (`GameplayStatics.GetGameMode`)))
  (set `/Game/Maps/CustomGameMode.HasBossyKey` true _ascustom_game_mode)
  (set `/Game/Maps/CustomGameMode.BossKeyNumber` 1 _ascustom_game_mode)
  (`self.K2_DestroyActor`)
  (`KismetSystemLibrary.PrintString` "You found a Boss Key!" true true (struct :`G` 0.020973 :`B` 0.4375 :`A` 1.0) 5.0))

(event `self.ReceiveTick`
  (params (DeltaSeconds :type "Float (single-precision)"))
  (bind _cube (`self.Cube`))
  (bind _floatdistance (`self.FloatDistance`))
  (bind (_returnvalue_x _returnvalue_y) (`KismetMathLibrary.BreakVector` (`SceneComponent.K2_GetComponentLocation` _cube)))
  (bind (_returnvalue_roll _returnvalue_pitch _returnvalue_yaw) (`KismetMathLibrary.BreakRotator` (`SceneComponent.K2_GetComponentRotation` (`self.Cube`))))
  (`SceneComponent.K2_SetWorldLocationAndRotation` _cube (`KismetMathLibrary.MakeVector` _returnvalue_x _returnvalue_y (+ (* (`KismetMathLibrary.DegCos` (* (/ (`self.Count`) (`self.FloatTotalTime`)) 360.0)) _floatdistance) _floatdistance (`self.Offset`))) (`KismetMathLibrary.MakeRotator` 0.0 0.0 (+ (* DeltaSeconds (`self.RotationSpeed`)) _returnvalue_yaw)) false false)
  (bind _output_get (set `self.Count` (+ (`self.Count`) DeltaSeconds)))
  (if (>= _output_get (`self.FloatTotalTime`))
    (set `self.Count` 0.0)))

(fn `UserConstructionScript`)