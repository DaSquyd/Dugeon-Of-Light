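; KeyItem is a pickup actor that floats and spins until a BP_Player overlaps it, then hovers above the player.
; While uncollected, Tick spins the Cube and bobs it on a looping cosine wave in world Z, based on Offset rather than its placed height.
; The overlap sets Collected, which stops that animation and makes Tick snap the actor above the first player's pawn each frame, matching its yaw.
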(event `self.ReceiveActorBeginOverlap`
  (params (OtherActor :type "Actor Object Reference"))
  (if (`self.Collected`)
    _
    (elif (== (`GameplayStatics.GetObjectClass` OtherActor) "/Game/Blueprints/Player/BP_Player.BP_Player_C")
      (set `self.Collected` true))))

(event `self.ReceiveTick`
  (params (DeltaSeconds :type "Float (single-precision)"))
  (bind _returnvalue (`GameplayStatics.GetPlayerPawn` 0))
  (bind _cube (`self.Cube`))
  (bind _floatdistance (`self.FloatDistance`))
  (bind (_returnvalue_x _returnvalue_y) (`KismetMathLibrary.BreakVector` (`SceneComponent.K2_GetComponentLocation` _cube)))
  (bind (_returnvalue_roll _returnvalue_pitch _returnvalue_yaw) (`KismetMathLibrary.BreakRotator` (`self.K2_GetActorRotation` _returnvalue)))
  (bind (_returnvalue_roll_2 _returnvalue_pitch_2 _returnvalue_yaw_2) (`KismetMathLibrary.BreakRotator` (`SceneComponent.K2_GetComponentRotation` (`self.Cube`))))
  (if (not (`self.Collected`))
    (`SceneComponent.K2_SetWorldLocationAndRotation` _cube (`KismetMathLibrary.MakeVector` _returnvalue_x _returnvalue_y (+ (* (`KismetMathLibrary.DegCos` (* (/ (`self.Count`) (`self.FloatTotalTime`)) 360.0)) _floatdistance) _floatdistance (`self.Offset`))) (`KismetMathLibrary.MakeRotator` 0.0 0.0 (+ (* DeltaSeconds (`self.RotationSpeed`)) _returnvalue_yaw_2)) false false)
    (bind _output_get (set `self.Count` (+ (`self.Count`) DeltaSeconds)))
    (if (>= _output_get (`self.FloatTotalTime`))
      (set `self.Count` 0.0)))
  (`/Engine/EditorBlueprintResources/StandardMacros.IsValid` _returnvalue
    (:`Is Valid`
      (if (`self.Collected`)
        (`self.K2_SetActorLocationAndRotation` (+ (`self.K2_GetActorLocation` _returnvalue) (0.0 0.0 200.0)) (`KismetMathLibrary.MakeRotator` 0.0 0.0 _returnvalue_yaw))))))

(fn `UserConstructionScript`)