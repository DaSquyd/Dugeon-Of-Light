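; Torch key item pickup that the player collects by walking into it.
; Overlap with an actor of exactly the BP_Player class sets a Collected flag.
; While the flag is set, Tick repeatedly hides the cube, disables cube and box collision, and snap-attaches the torch to player pawn 0.
; A forward local-offset node is left unconnected and flagged as a problem, so it never runs.
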(event `self.ReceiveActorBeginOverlap`
  (params (OtherActor :type "Actor Object Reference"))
  (if (`self.Collected`)
    _
    (elif (== (`GameplayStatics.GetObjectClass` OtherActor) "/Game/Blueprints/Player/BP_Player.BP_Player_C")
      (set `self.Collected` true))))

(event `self.ReceiveTick`
  (params (DeltaSeconds :type "Float (single-precision)"))
  (bind _returnvalue (`GameplayStatics.GetPlayerPawn` 0))
  (`/Engine/EditorBlueprintResources/StandardMacros.IsValid` _returnvalue
    (:`Is Valid`
      (if (`self.Collected`)
        (`|ExecutionSequence`
          (:`then_0`
            (`SceneComponent.SetVisibility` (`self.Cube`) false false)
            (`PrimitiveComponent.SetCollisionEnabled` (`self.Cube`) "NoCollision")
            (`PrimitiveComponent.SetCollisionEnabled` (`self.Box`) "NoCollision"))
          (:`then_1`
            (`self.K2_AttachToActor` _returnvalue "None" "SnapToTarget" "SnapToTarget" "SnapToTarget")))))))

(fn `UserConstructionScript`)