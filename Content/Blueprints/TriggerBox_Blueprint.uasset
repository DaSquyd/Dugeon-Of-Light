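; Trigger box that starts a boss fight when the player overlaps it.
; If the custom game mode's FightingBoss flag is not already set, it calls Spawn on its Spawner and moves BossDoor back to its initial location.
; It then sets FightingBoss on the game mode, so further overlaps do nothing while that flag stays true.
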(event `self.ReceiveActorBeginOverlap`
  (params (OtherActor :type "Actor Object Reference"))
  (bind _bossdoor (`self.BossDoor`))
  (bind _ascustom_game_mode (cast `/Game/Maps/CustomGameMode` (`GameplayStatics.GetGameMode`)))
  (if (not (`/Game/Maps/CustomGameMode.FightingBoss` _ascustom_game_mode))
    (cast `/Game/Blueprints/Player/BP_Player` OtherActor)
    (`/Game/Blueprints/Enemies/Spawner.Spawn` (`self.Spawner`))
    (`SceneComponent.K2_SetWorldLocation` (`Actor.RootComponent` _bossdoor) (`/Game/Blueprints/LightObjects/BossDoor.initialLocation` _bossdoor) false false)
    (bind _ascustom_game_mode_2 (cast `/Game/Maps/CustomGameMode` (`GameplayStatics.GetGameMode`)))
    (set `/Game/Maps/CustomGameMode.FightingBoss` true _ascustom_game_mode_2)))

(fn `UserConstructionScript`)