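; BP_Player is the player pawn, with walk, strafe, jump, yaw-only aim, a ranged shot and a melee attack.
; Shooting spends ammo to spawn a BP_Bullet at the player's location and yaw, then waits out a Delay cooldown.
; The attack damages every actor overlapping AttackCollider.
; Its cooldown and brief AttackDisplay flash run inside that loop, so they only trigger when something overlaps.
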(event `InputAction|Jump`
  (params (Key :type "Key Structure"))
  (:`Pressed`
    (`self.Jump`)))

(event `InputAxis|Walk`
  (params (AxisValue :type "Float (single-precision)"))
  (`self.AddMovementInput` (`self.GetActorForwardVector`) AxisValue))

(event `InputAxis|Strafe`
  (params (AxisValue :type "Float (single-precision)"))
  (`self.AddMovementInput` (`self.GetActorRightVector`) AxisValue))

(event `InputAxis|Aim`
  (params (AxisValue :type "Float (single-precision)"))
  (`self.AddControllerYawInput` AxisValue))

(event `InputAction|Shoot`
  (params (Key :type "Key Structure"))
  (bind _returnvalue (`self.GetTransform`))
  (:`Pressed`
    (if (and (`self.CanShoot`) (> (`self.Ammo`) 0))
      (`|SpawnActorFromClass` "/Game/Blueprints/Projectile/BP_Bullet.BP_Bullet_C" (`KismetMathLibrary.MakeTransform` (.location _returnvalue) (`KismetMathLibrary.MakeRotator` 0.0 0.0 (.yaw (.rotation _returnvalue)))) "Undefined" "OverrideRootScale" null null)
      (set `self.CanShoot` false)
      (`/Engine/EditorBlueprintResources/StandardMacros.DecrementInt` (`self.Ammo`)
        (:`  `
          (`KismetSystemLibrary.Delay` 1.0)
          (set `self.CanShoot` true))))))

(event `InputAction|Attack`
  (params (Key :type "Key Structure"))
  (:`Pressed`
    (if (`self.CanAttack`)
      (for _array_element (`PrimitiveComponent.GetOverlappingActors` (`self.AttackCollider`) null)
        (`GameplayStatics.ApplyDamage` _array_element 5.0 null self)
        (`|ExecutionSequence`
          (:`then_0`
            (set `self.CanAttack` false)
            (`KismetSystemLibrary.Delay` 0.5)
            (set `self.CanAttack` true))
          (:`then_1`
            (`SceneComponent.SetVisibility` (`self.AttackDisplay`) true false)
            (`KismetSystemLibrary.Delay` 0.1)
            (`SceneComponent.SetVisibility` (`self.AttackDisplay`) false false)))))))

(fn `UserConstructionScript`)