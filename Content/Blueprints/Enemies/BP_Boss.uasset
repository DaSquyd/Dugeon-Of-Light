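; Boss enemy that fights the player while AI perception senses them, mirroring sight to a Blackboard key.
; A looping timer randomly re-rolls its state every 1–2 seconds, and Tick runs it.
; It chases via AIMoveTo, fires bullets on a cooldown, or charges using a physics capsule impulse with boosted melee damage.
; The roll only spans the first three options, so it never selects Charge.
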(event `self.ReceiveBeginPlay`
  (`self.SetState`))

(event `SetState`
  (`KismetSystemLibrary.Delay` (`KismetMathLibrary.RandomFloatInRange` 1.0 2.0))
  (set `self.State` (select `int` (`KismetMathLibrary.RandomInteger` 3) :`0` "NewEnumerator0" :`1` "NewEnumerator1" :`2` "NewEnumerator1" :`3` "NewEnumerator2" :`4` "NewEnumerator2" :!type "/Game/Blueprints/Enemies/EBossState Enum"))
  (`self.SetState`))

(event `self.ReceiveTick`
  (params (DeltaSeconds :type "Float (single-precision)"))
  (bind _returnvalue (`GameplayStatics.GetPlayerCharacter` 0))
  (bind _returnvalue_2 (`self.GetTransform`))
  (bind _returnvalue_3 (`GameplayStatics.GetPlayerCharacter` 0))
  (bind (_returnvalue_x _returnvalue_y) (`KismetMathLibrary.BreakVector` (* (`self.GetActorForwardVector`) 3000.0)))
  (bind (_returnvalue_roll _returnvalue_pitch _returnvalue_yaw) (`KismetMathLibrary.BreakRotator` (`KismetMathLibrary.FindLookAtRotation` (`self.K2_GetActorLocation`) (`self.K2_GetActorLocation` _returnvalue))))
  (`parent.ReceiveTick` DeltaSeconds)
  (if (`self.Aggressive`)
    (switch `/Game/Blueprints/Enemies/EBossState` (`self.State`)
      (:`NewEnumerator0`
        (`|AIMoveTo` self (0.0 0.0 0.0) (`GameplayStatics.GetPlayerCharacter` 0) 50.0
          (:`then`
            (`PrimitiveComponent.SetSimulatePhysics` (`self.CapsuleComponent`) false))))
      (:`NewEnumerator1`
        (`|ExecutionSequence`
          (:`then_0`
            (`/Engine/EditorBlueprintResources/StandardMacros.IsValid` _returnvalue
              (:`Is Valid`
                (`self.K2_SetActorRotation` (`KismetMathLibrary.MakeRotator` 0.0 0.0 _returnvalue_yaw))
                (set `self.IsShooting` true))))
          (:`then_1`
            (if (and (`self.IsShooting`) (not (`self.HasShot`)))
              (bind _returnvalue_4 (`|SpawnActorFromClass` "/Game/Blueprints/Enemies/BP_BulletEnemy.BP_BulletEnemy_C" (`KismetMathLibrary.MakeTransform` (`KismetMathLibrary.MakeVector` (.x (.location _returnvalue_2)) (.y (.location _returnvalue_2)) (- (.z (.location _returnvalue_2)) 100.0)) (`KismetMathLibrary.MakeRotator` 0.0 0.0 (.yaw (.rotation _returnvalue_2)))) "Undefined" "OverrideRootScale" null null))
              (set `/Game/Blueprints/Enemies/BP_BulletEnemy.Damage` 40.0 _returnvalue_4)
              (set `self.HasShot` true)
              (set `self.IsShooting` false)
              (`KismetSystemLibrary.Delay` 4.0)
              (set `self.HasShot` false)))))
      (:`NewEnumerator2`
        (if (not (`self.IsCharging`))
          (`/Engine/EditorBlueprintResources/StandardMacros.IsValid` _returnvalue_3
            (:`Is Valid`
              (`self.K2_SetActorRotation` (`KismetMathLibrary.FindLookAtRotation` (`self.K2_GetActorLocation`) (`self.K2_GetActorLocation` _returnvalue_3)))
              (`PrimitiveComponent.SetSimulatePhysics` (`self.CapsuleComponent`) true)
              (set `self.MeleeDamage` 75.0)
              (`KismetSystemLibrary.Delay` 2.0)
              (set `self.IsCharging` true)
              (`PrimitiveComponent.AddImpulse` (`self.CapsuleComponent`) (`KismetMathLibrary.MakeVector` _returnvalue_x _returnvalue_y -100.0) "None" true)
              (set `self.Direction` (`KismetMathLibrary.Vector_Normal2D` (`KismetMathLibrary.MakeVector` _returnvalue_x _returnvalue_y -100.0)))
              (`KismetSystemLibrary.Delay` 3.0)
              (set `self.IsCharging` false)
              (set `self.MeleeDamage` 30.0))))))
    (else
      (`PrimitiveComponent.SetSimulatePhysics` (`self.CapsuleComponent`) false))))

(event `self.AIPerception.OnTargetPerceptionUpdated`
  (params (Actor :type "Actor Object Reference") (Stimulus :type "AIStimulus Structure"))
  (bind (_age _expirationage _strength _stimuluslocation _receiverlocation _tag _bsuccessfullysensed) (break `AIStimulus` Stimulus))
  (cast `/Game/Blueprints/Player/BP_Player` Actor)
  (`BlackboardComponent.SetValueAsBool` (`AIBlueprintHelperLibrary.GetBlackboard` null) "CanSeePlayer" _bsuccessfullysensed)
  (set `self.Aggressive` _bsuccessfullysensed))

(fn `UserConstructionScript`
  (`parent.UserConstructionScript`)
  (set `self.MeleeDamage` 25.0)
  (set `CharacterMovementComponent.MaxWalkSpeed` (`self.WalkSpeed`) (`self.CharacterMovement`)))