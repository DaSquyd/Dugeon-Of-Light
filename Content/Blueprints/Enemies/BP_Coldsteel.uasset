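; Coldsteel enemy that chases the player and periodically teleports behind them.
; When neither patrolling nor readying, Tick issues an AI MoveTo toward the player and immediately sets Readying, without waiting for arrival.
; After a delay it teleports just behind the player pawn's forward vector and copies the player's rotation.
; A second delay acts as a cooldown before Readying clears and the cycle can repeat.
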(event `self.ReceiveTick`
  (params (DeltaSeconds :type "Float (single-precision)"))
  (bind _returnvalue (`GameplayStatics.GetPlayerPawn` 0))
  (`parent.ReceiveTick` DeltaSeconds)
  (`|ExecutionSequence`
    (:`then_0`
      (if (not (or (`self.IsPatrolling`) (`self.Readying`)))
        (`|AIMoveTo` self (0.0 0.0 0.0) (`GameplayStatics.GetPlayerCharacter` 0) 50.0
          (:`then`
            (set `self.Readying` true)
            (`KismetSystemLibrary.Delay` 3.0)
            (`self.K2_TeleportTo` (- (`self.K2_GetActorLocation` _returnvalue) (* (`self.GetActorForwardVector` _returnvalue) 50.0)))
            (`self.K2_SetActorRotation` (`self.K2_GetActorRotation` (`GameplayStatics.GetPlayerPawn` 0)))
            (`KismetSystemLibrary.Delay` 5.0)
            (set `self.Readying` false)))))))

(fn `UserConstructionScript`
  (`parent.UserConstructionScript`))