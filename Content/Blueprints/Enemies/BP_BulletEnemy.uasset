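; BP_BulletEnemy is an enemy bullet actor that damages the player.
; Overlapping an actor whose class is exactly BP_Player makes it destroy itself, then apply its Damage value to that actor.
; A hit on its Sphere component also destroys it without applying damage, and a timer started on BeginPlay removes it after a fixed lifetime.
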(event `self.ReceiveActorBeginOverlap`
  (params (OtherActor :type "Actor Object Reference"))
  (if (== (`GameplayStatics.GetObjectClass` OtherActor) "/Game/Blueprints/Player/BP_Player.BP_Player_C")
    (`self.K2_DestroyActor`)
    (`GameplayStatics.ApplyDamage` OtherActor (`self.Damage`))))

(event `self.ReceiveBeginPlay`
  (`KismetSystemLibrary.Delay` 5.0)
  (`self.K2_DestroyActor`))

(event `self.Sphere.OnComponentHit`
  (params (HitComponent :type "PrimitiveComponent Object Reference") (OtherActor :type "Actor Object Reference") (OtherComp :type "PrimitiveComponent Object Reference") (NormalImpulse :type "Vector Structure") (Hit :type "HitResult Structure (by ref)"))
  (`self.K2_DestroyActor`))

(fn `UserConstructionScript`)