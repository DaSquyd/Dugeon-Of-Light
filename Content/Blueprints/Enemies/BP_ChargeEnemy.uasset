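; Charging enemy Blueprint that chases the player and periodically lunges forward.
; When neither patrolling nor charging, Tick issues an AI move to the player's location and starts a delayed charge sequence without waiting for arrival.
; During the timed charge, Tick offsets the actor along its forward vector without sweep, by a per-frame Speed that decays with delta time.
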(event `self.ReceiveTick`
  (params (DeltaSeconds :type "Float (single-precision)"))
  (`parent.ReceiveTick` DeltaSeconds)
  (`|ExecutionSequence`
    (:`then_0`
      (if (not (or (`self.IsPatrolling`) (`self.IsCharging`)))
        (`|AIMoveTo` self (`self.K2_GetActorLocation` (`GameplayStatics.GetPlayerCharacter` 0)) null 50.0
          (:`then`
            (`KismetSystemLibrary.Delay` 2.0)
            (set `self.IsCharging` true)
            (set `self.Speed` 15.0)
            (`KismetSystemLibrary.Delay` 3.0)
            (set `self.IsCharging` false)))))
    (:`then_1`
      (if (`self.IsCharging`)
        (`self.K2_AddActorWorldOffset` (* (`self.GetActorForwardVector`) (`self.Speed`)))
        (set `self.Speed` (- (`self.Speed`) (* 5.0 DeltaSeconds)))))))

(fn `UserConstructionScript`
  (`parent.UserConstructionScript`))