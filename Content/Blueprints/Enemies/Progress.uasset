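; Behavior tree task that advances a looping timer in an enemy's blackboard.
; Each execution adds world delta time scaled by Multiplier to Count, prints a progress value and finishes successfully at once.
; Count resets upon reaching TargetTime.
; The threshold test re-reads Count after each write, so the Bool key is evaluated after any reset and normally stays false.
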(event `self.ReceiveExecuteAI`
  (params (OwnerController :type "AIController Object Reference") (ControlledPawn :type "Pawn Object Reference"))
  (bind _count (`self.Count`))
  (bind _returnvalue (+ (`BTFunctionLibrary.GetBlackboardValueAsFloat` _count) (* (`GameplayStatics.GetWorldDeltaSeconds`) (`self.Multiplier`))))
  (bind _returnvalue_2 (>= _returnvalue (`self.TargetTime`)))
  (`BTFunctionLibrary.SetBlackboardValueAsFloat` _count _returnvalue)
  (`KismetSystemLibrary.PrintString` (`KismetStringLibrary.Conv_DoubleToString` _returnvalue))
  (if _returnvalue_2
    (`BTFunctionLibrary.SetBlackboardValueAsFloat` (`self.Count`)))
  (`BTFunctionLibrary.SetBlackboardValueAsBool` (`self.Bool`) _returnvalue_2)
  (`self.FinishExecute` true))