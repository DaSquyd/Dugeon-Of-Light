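; ChargePlayer is a Behavior Tree task for enemy AI, named for a charge at the player, though it contains no movement or attack logic.
; On AI execute, it copies the Charging and Preparing flags and the Direction vector from the owner controller's Blackboard into variables.
; It then immediately finishes as failed, without using those values or writing anything back to the Blackboard.
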(event `self.ReceiveExecuteAI`
  (params (OwnerController :type "AIController Object Reference") (ControlledPawn :type "Pawn Object Reference"))
  (bind _returnvalue (`AIBlueprintHelperLibrary.GetBlackboard` OwnerController))
  (set `self.IsCharging` (`BlackboardComponent.GetValueAsBool` _returnvalue "Charging"))
  (set `self.Preparing` (`BlackboardComponent.GetValueAsBool` _returnvalue "Preparing"))
  (set `self.Direction` (`BlackboardComponent.GetValueAsVector` _returnvalue "Direction"))
  (`self.FinishExecute` false))