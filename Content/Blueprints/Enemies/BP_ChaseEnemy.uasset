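; Enemy Blueprint that chases the first player character whenever it is not patrolling.
; Tick reissues an AI Move To toward the player every frame and adds a small unswept forward offset, independent of frame time.
; Two hit-flash experiments, one using a dynamic material color and one toggling capsule visibility, are left unconnected and never run.
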(event `self.ReceiveTick`
  (params (DeltaSeconds :type "Float (single-precision)"))
  (`parent.ReceiveTick` DeltaSeconds)
  (if (not (`self.IsPatrolling`))
    (`|AIMoveTo` self (0.0 0.0 0.0) (`GameplayStatics.GetPlayerCharacter` 0) 50.0
      (:`then`
        (`self.K2_AddActorWorldOffset` (* (`self.GetActorForwardVector`) 2.0))))))

(fn `UserConstructionScript`
  (`parent.UserConstructionScript`))