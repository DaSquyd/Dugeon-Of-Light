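; Enemy that charges at the player with a physics impulse while it senses them.
; AI perception sets the aggression flag and a blackboard key; Tick then turns the enemy toward the player and launches it after a delay.
; Attacking is enabled during the timed charge.
; If its facing strays from the launch direction, Bounce knocks it backward and cancels the charge and attack.
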(event `self.ReceiveTick`
  (params (DeltaSeconds :type "Float (single-precision)"))
  (bind _returnvalue (`GameplayStatics.GetPlayerCharacter` 0))
  (bind _capsulecomponent (`self.CapsuleComponent`))
  (bind _returnvalue_2 (* (`self.GetActorForwardVector`) 3000.0))
  (`parent.ReceiveTick` DeltaSeconds)
  (`|ExecutionSequence`
    (:`then_0`
      (if (not (or (`self.IsCharging`) (not (`self.Aggressive_0`))))
        (`/Engine/EditorBlueprintResources/StandardMacros.IsValid` _returnvalue
          (:`Is Valid`
            (`self.K2_SetActorRotation` (`KismetMathLibrary.FindLookAtRotation` (`self.K2_GetActorLocation`) (`self.K2_GetActorLocation` _returnvalue)))
            (`KismetSystemLibrary.Delay` 4.0)
            (if (`self.Aggressive_0`)
              (set `self.IsCharging` true)
              (`PrimitiveComponent.SetSimulatePhysics` _capsulecomponent true)
              (`PrimitiveComponent.AddImpulse` _capsulecomponent _returnvalue_2 "None" true)
              (set `self.Direction` (`KismetMathLibrary.Vector_Normal2D` _returnvalue_2))
              (set `self.CanAttack` true)
              (`KismetSystemLibrary.Delay` 7.0)
              (set `self.IsCharging` false)
              (set `self.CanAttack` false)
              (`PrimitiveComponent.SetSimulatePhysics` (`self.CapsuleComponent`) false))))))
    (:`then_1`
      (if (and (`self.IsCharging`) (!= (`self.GetActorForwardVector`) (`KismetMathLibrary.Vector_Normal2D` (`self.Direction`)) :`ErrorTolerance` 1.0))
        (`self.Bounce`)))))

(event `self.ReceiveAnyDamage`
  (params (Damage :type "Float (single-precision)") (DamageType :type "DamageType Object Reference") (InstigatedBy :type "Controller Object Reference") (DamageCauser :type "Actor Object Reference")))

(event `Bounce`
  (`PrimitiveComponent.SetPhysicsLinearVelocity` (`self.CapsuleComponent`) (* (`self.GetActorForwardVector`) -500.0) false "None")
  (set `self.IsCharging` false)
  (set `self.CanAttack` false))

(event `self.AIPerception.OnTargetPerceptionUpdated`
  (params (Actor :type "Actor Object Reference") (Stimulus :type "AIStimulus Structure"))
  (bind (_age _expirationage _strength _stimuluslocation _receiverlocation _tag _bsuccessfullysensed) (break `AIStimulus` Stimulus))
  (cast `/Game/Blueprints/Player/BP_Player` Actor)
  (`BlackboardComponent.SetValueAsBool` (`AIBlueprintHelperLibrary.GetBlackboard` null) "CanSeePlayer" _bsuccessfullysensed)
  (set `self.Aggressive_0` _bsuccessfullysensed))

(fn `UserConstructionScript`
  (`parent.UserConstructionScript`)
  (set `self.CanAttack` false))