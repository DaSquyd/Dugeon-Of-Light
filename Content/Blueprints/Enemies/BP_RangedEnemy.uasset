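; Ranged enemy that, while its AI perception senses BP_Player, turns to face the player and fires BP_BulletEnemy shots on a cooldown.
; Perception updates set the CanSeePlayer blackboard key, the aggression flag and capsule physics simulation.
; Tick drives aiming, delayed firing and velocity-based movement: backing away harder the closer the player is, or strafing randomly left or right when out of range.
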(event `self.ReceiveTick`
  (params (DeltaSeconds :type "Float (single-precision)"))
  (bind _returnvalue (`self.GetTransform`))
  (bind _returnvalue_2 (`KismetMathLibrary.Vector_Distance2D` (`self.K2_GetActorLocation`) (`self.K2_GetActorLocation` (`GameplayStatics.GetPlayerPawn` 0))))
  (`parent.ReceiveTick` DeltaSeconds)
  (`|ExecutionSequence`
    (:`then_0`
      (if (`self.Aggressive_0`)
        (`self.K2_SetActorRotation` (`KismetMathLibrary.FindLookAtRotation` (`self.K2_GetActorLocation`) (`self.K2_GetActorLocation` (`GameplayStatics.GetPlayerCharacter` 0))))
        (set `self.IsShooting` true)))
    (:`then_1`
      (`KismetSystemLibrary.Delay` 0.2)
      (if (and (`self.IsShooting`) (not (`self.HasShot`)) (`self.Aggressive_0`))
        (bind _returnvalue_3 (`|SpawnActorFromClass` "/Game/Blueprints/Enemies/BP_BulletEnemy.BP_BulletEnemy_C" (`KismetMathLibrary.MakeTransform` (.location _returnvalue) (`KismetMathLibrary.MakeRotator` 0.0 0.0 (.yaw (.rotation _returnvalue)))) "Undefined" "OverrideRootScale" null null))
        (`/Engine/EditorBlueprintResources/StandardMacros.IsValid` _returnvalue_3
          (:`Is Valid`
            (set `/Game/Blueprints/Enemies/BP_BulletEnemy.Damage` 10.0 _returnvalue_3)
            (set `self.HasShot` true)
            (set `self.IsShooting` false)
            (`KismetSystemLibrary.Delay` 1.0)
            (set `self.HasShot` false)))))
    (:`then_2`
      (`/Engine/EditorBlueprintResources/StandardMacros.IsValid` (`GameplayStatics.GetPlayerPawn` 0)
        (:`Is Valid`
          (if (and (`self.IsShooting`) (`self.Aggressive_0`))
            (if (<= _returnvalue_2 1000.0)
              (`PrimitiveComponent.SetAllPhysicsLinearVelocity` (`self.CapsuleComponent`) (* (`self.GetActorForwardVector`) (* (- 1000.0 _returnvalue_2) -0.5)) false)
              (else
                (`self.Shuffle`)))))))))

(event `Shuffle`
  (bind _returnvalue (`self.GetActorRightVector`))
  (bind _capsulecomponent (`self.CapsuleComponent`))
  (if (not (`self.Shuffling`))
    (`|ExecutionSequence`
      (:`then_0`
        (if (`KismetMathLibrary.RandomBool`)
          (`PrimitiveComponent.SetPhysicsLinearVelocity` _capsulecomponent (* _returnvalue 600.0) false "None")
          (else
            (`PrimitiveComponent.SetPhysicsLinearVelocity` _capsulecomponent (* _returnvalue -600.0) false "None"))))
      (:`then_1`
        (set `self.Shuffling` true)
        (`KismetSystemLibrary.Delay` (`KismetMathLibrary.RandomFloatInRange` 0.5 2.0))
        (if (`self.IsShooting`)
          (set `self.Shuffling` false))))))

(event `self.AIPerception.OnTargetPerceptionUpdated`
  (params (Actor :type "Actor Object Reference") (Stimulus :type "AIStimulus Structure"))
  (bind (_age _expirationage _strength _stimuluslocation _receiverlocation _tag _bsuccessfullysensed) (break `AIStimulus` Stimulus))
  (cast `/Game/Blueprints/Player/BP_Player` Actor)
  (`BlackboardComponent.SetValueAsBool` (`AIBlueprintHelperLibrary.GetBlackboard` null) "CanSeePlayer" _bsuccessfullysensed)
  (set `self.Aggressive_0` _bsuccessfullysensed)
  (`PrimitiveComponent.SetSimulatePhysics` (`self.CapsuleComponent`) _bsuccessfullysensed))

(fn `UserConstructionScript`
  (`parent.UserConstructionScript`))